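; Enemy character Blueprint with an HP pool, a world health bar widget and a reusable death-and-reset cycle.
; It starts with its AI controller unpossessed; CastedEvent shows the mesh and widget, then possesses it.
; AnyDamage updates the bar and calls Death at zero, which unpossesses, waits, teleports to the start transform, hides the mesh and restores HP.
; Tick shows the bar only while the player is nearby.
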(event `self.ReceiveBeginPlay`
  (set `self.Start Transform` (`self.GetTransform`))
  (bind _output_get (set `self.Ai Controller` (`AIBlueprintHelperLibrary.GetAIController` self)))
  (`Controller.UnPossess` _output_get)
  (set `/Game/Blueprints/Health_Bar_Enemy.Health` (/ (`self.HP`) (`self.Max HP`)) (cast `/Game/Blueprints/Health_Bar_Enemy` (`WidgetComponent.GetWidget` (`self.Widget`)) :!pure true)))

(event `self.ReceiveTick`
  (params (DeltaSeconds :type "Float (single-precision)"))
  (bind _widget (`self.Widget`))
  (if (<= (`self.GetDistanceTo` (`GameplayStatics.GetPlayerCharacter` 0)) 800.0)
    (`SceneComponent.SetVisibility` _widget true false)
    (else
      (`SceneComponent.SetVisibility` _widget false false))))

(event `Casted Event`
  (`SceneComponent.SetVisibility` (`self.Mesh`) true false)
  (`SceneComponent.SetVisibility` (`self.Widget`) true false)
  (set `self.Called` true)
  (`Controller.Possess` (`self.Ai Controller`) self))

(event `Death`
  (bind (_start_transform_location _start_transform_rotation) (`KismetMathLibrary.BreakTransform` (`self.Start Transform`)))
  (`Controller.UnPossess` (`self.Ai Controller`))
  (set `self.Called` false)
  (`KismetSystemLibrary.Delay` 5.0)
  (`self.K2_TeleportTo` _start_transform_location _start_transform_rotation)
  (`SceneComponent.SetVisibility` (`self.Mesh`) false false)
  (set `self.HP` (`self.Max HP`)))

(event `self.ReceiveAnyDamage`
  (params (Damage :type "Float (single-precision)") (DamageType :type "DamageType Object Reference") (InstigatedBy :type "Controller Object Reference") (DamageCauser :type "Actor Object Reference"))
  (bind _returnvalue (- (`self.HP`) Damage))
  (bind _ashealth_bar_enemy (cast `/Game/Blueprints/Health_Bar_Enemy` (`WidgetComponent.GetWidget` (`self.Widget`)) :!pure true))
  (if (<= _returnvalue 0.0)
    (set `/Game/Blueprints/Health_Bar_Enemy.Health` 0.0 _ashealth_bar_enemy)
    (`self.Death`)
    (else
      (set `self.HP` _returnvalue)
      (set `/Game/Blueprints/Health_Bar_Enemy.Health` (/ (`self.HP`) (`self.Max HP`)) _ashealth_bar_enemy))))

(fn `UserConstructionScript`)
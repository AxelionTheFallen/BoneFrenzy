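; Wave manager that spawns enemies in timed waves inside a box, driven by rows of a wave data table.
; BeginPlay loads the rows and starts ProgressWave, which spawns each wave with row-defined stats and re-arms a timer until the row's wave count is reached, then increments the row index.
; Spawn points are re-rolled recursively until clear of the player.
; SpawnWave resets counters but is uncalled here; CheckForWave is a stub.
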(event `self.ReceiveBeginPlay`
  (bind _outrownames (`DataTableFunctionLibrary.GetDataTableRowNames` "/Game/Blueprints/Enemy/wavedata.wavedata"))
  (for _array_element _outrownames
    (bind _returnvalue (`|GetDataTableRow` "/Game/Blueprints/Enemy/wavedata.wavedata" _array_element)
      (:`then`
        (`KismetArrayLibrary.Array_Add` (`self.WaveDatas`) _returnvalue))))
  (`self.ProgressWave`))

(fn `CheckForWave`
  (if (== (`self.EnemyAmount`) 0)
    _))

(fn `GetSpawnEnemyLocation`
  (returns (Location :type "Vector Structure"))
  (locals (`L-Location` :type "Vector Structure" :default (0.0 0.0 0.0)))
  (bind (_origin _boxextent) (`KismetSystemLibrary.GetComponentBounds` (`self.Box`)))
  (bind _output_get (set `local.L-Location` (`KismetMathLibrary.RandomPointInBoundingBox` _origin _boxextent)))
  (if (> (`KismetMathLibrary.Vector_Distance` _output_get (`self.K2_GetActorLocation` (`GameplayStatics.GetPlayerCharacter` 0))) 500.0)
    (return (`local.L-Location`))
    (else
      (return (`self.GetSpawnEnemyLocation`)))))

(fn `ProgressWave`
  (bind (_enemyperwave _waveamount _timebetweenwaves _hp _damage) (break `/Game/Blueprints/Enemy/Wavestruct` (`|GetArrayItem` (`self.WaveDatas`) (`self.WaveIndex`))))
  (`/Engine/EditorBlueprintResources/StandardMacros.IncrementInt` (`self.CurrentWave`)
    (:`  `
      (for _ (range 1 (+ _enemyperwave 1))
        (`self.SpawnEnemy` _hp _damage))
      (if (== _waveamount (`self.CurrentWave`))
        (`/Engine/EditorBlueprintResources/StandardMacros.IncrementInt` (`self.WaveIndex`))
        (else
          (`KismetSystemLibrary.K2_SetTimer` null "ProgressWave" _timebetweenwaves))))))

(fn `SpawnEnemy`
  (params (EnemyHP :type "Float (double-precision)") (EnemyDamage :type "Float (double-precision)"))
  (`|SpawnActorFromClass` "/Game/Blueprints/Enemy/Enemy.Enemy_C" (`KismetMathLibrary.MakeTransform` (`self.GetSpawnEnemyLocation`)) "Undefined" "MultiplyWithRoot" null EnemyHP EnemyDamage self null))

(fn `SpawnWave`
  (bind (_enemyperwave _waveamount) (break `/Game/Blueprints/Enemy/Wavestruct` (`|GetArrayItem` (`self.WaveDatas`) (`self.WaveIndex`))))
  (set `self.CurrentWave` 0)
  (set `self.EnemyAmount` (* _enemyperwave _waveamount))
  (`self.ProgressWave`))

(fn `UserConstructionScript`)
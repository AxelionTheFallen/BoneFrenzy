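; Enemy character with health that gets knocked back and damaged when hit, and reports its death to a wave manager.
; PushEnemy always launches it away from the hit location, but applies damage only when CanTakeDamage is set, followed by a one-second invulnerability window.
; Surviving hits update the health bar widget cached at BeginPlay.
; At zero HP it decrements the Manager's enemy count, triggers the wave check, plays a break sound and destroys itself.
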(event `self.ReceiveBeginPlay`
  (bind _ashealth_bar_enemy (cast `/Game/Blueprints/Widgets/Health_Bar_Enemy` (`WidgetComponent.GetWidget` (`self.Widget`))))
  (set `self.HPBar` _ashealth_bar_enemy)
  (set `self.HP` (`self.Max HP`)))

(event `/Game/Blueprints/BPI_Push.PushEnemy`
  (params (Damage :type "Float (double-precision)") (HitLocation :type "Vector Structure"))
  (bind _manager (`self.Manager`))
  (`self.LaunchCharacter` (* 3000.0 (`KismetMathLibrary.FindLookAtRotation` HitLocation (`self.K2_GetActorLocation`))) true true)
  (if (`self.CanTakeDamage`)
    (set `self.CanTakeDamage` false)
    (bind _output_get (set `self.HP` (- (`self.HP`) Damage)))
    (if (<= _output_get 0.0)
      (set `/Game/Blueprints/Enemy/BP_WaveManager.EnemyAmount` (- (`/Game/Blueprints/Enemy/BP_WaveManager.EnemyAmount` _manager) 1) _manager)
      (`/Game/Blueprints/Enemy/BP_WaveManager.CheckForWave` (`self.Manager`))
      (`GameplayStatics.SpawnSound2D` "/Game/Blueprints/EnemyBreak_SoundEffect.EnemyBreak_SoundEffect" 0.2 1.0 0.0 null)
      (`self.K2_DestroyActor`)
      (else
        (`ProgressBar.SetPercent` (`/Game/Blueprints/Widgets/Health_Bar_Enemy.ProgressBar_102` (`self.HPBar`)) (/ (`self.HP`) (`self.Max HP`)))
        (`KismetSystemLibrary.Delay` 1.0)
        (set `self.CanTakeDamage` true)))))

(fn `UserConstructionScript`)
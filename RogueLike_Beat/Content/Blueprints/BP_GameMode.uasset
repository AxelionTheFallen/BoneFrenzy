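; Game mode that continuously spawns enemies around the player by recycling Enemy actors gathered at BeginPlay.
; A self-recursing SpawnEnemy loop with delays picks a random point in one of four bands surrounding the player.
; It treats hidden meshes as free pool slots within MaxEnemySpawnValue, retrying later when none are free.
; A free enemy teleports to a random navigable point near that location, then receives CastedEvent.
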(event `self.ReceiveBeginPlay`
  (bind _outactors (`GameplayStatics.GetAllActorsOfClass` "/Game/Blueprints/Enemy/Enemy.Enemy_C"))
  (set `self.Out Actors` _outactors)
  (`KismetSystemLibrary.Delay` 3.0)
  (`self.Spawn Enemy`))

(event `Spawn Enemy`
  (bind _returnvalue (`GameplayStatics.GetPlayerCharacter` 0))
  (bind _current_enemy (`self.Current Enemy`))
  (bind (_returnvalue_x _returnvalue_y _returnvalue_z) (`KismetMathLibrary.BreakVector` (`self.K2_GetActorLocation` _returnvalue)))
  (bind _returnvalue_2 (+ _returnvalue_y 1800.0))
  (bind _returnvalue_3 (- _returnvalue_y 1800.0))
  (bind _returnvalue_4 (- _returnvalue_x 1800.0))
  (bind _returnvalue_5 (+ _returnvalue_x 1800.0))
  (`/Engine/EditorBlueprintResources/StandardMacros.IsValid` _returnvalue
    (:`Is Valid`
      (`|ExecutionSequence`
        (:`then_0`
          (switch `int` (`KismetMathLibrary.RandomIntegerInRange` 0 4)
            (:`0`
              (set `self.Teleport Location` (`KismetMathLibrary.MakeVector` (`KismetMathLibrary.RandomFloatInRange` _returnvalue_4 _returnvalue_5) (`KismetMathLibrary.RandomFloatInRange` _returnvalue_3 (- _returnvalue_y 1400.0)) _returnvalue_z)))
            (:`1`
              (set `self.Teleport Location` (`KismetMathLibrary.MakeVector` (`KismetMathLibrary.RandomFloatInRange` _returnvalue_4 _returnvalue_5) (`KismetMathLibrary.RandomFloatInRange` (+ _returnvalue_y 1400.0) _returnvalue_2) _returnvalue_z)))
            (:`2`
              (set `self.Teleport Location` (`KismetMathLibrary.MakeVector` (`KismetMathLibrary.RandomFloatInRange` _returnvalue_4 (- _returnvalue_x 1400.0)) (`KismetMathLibrary.RandomFloatInRange` _returnvalue_3 _returnvalue_2) _returnvalue_z)))
            (:`3`
              (set `self.Teleport Location` (`KismetMathLibrary.MakeVector` (`KismetMathLibrary.RandomFloatInRange` (+ _returnvalue_x 1400.0) _returnvalue_5) (`KismetMathLibrary.RandomFloatInRange` _returnvalue_3 _returnvalue_2) _returnvalue_z)))))
        (:`then_1`
          (for (_array_element _array_index) (`self.Out Actors`)
            (if (< _array_index (`self.Max Enemy Spawn Value`))
              (if (`SceneComponent.IsVisible` (`Character.Mesh` _array_element))
                (set `self.On Spawn Limit` true)
                (set `self.Current Enemy` null)
                (else
                  (set `self.On Spawn Limit` false)
                  (set `self.Current Enemy` _array_element)
                  (break)))
              (else
                (set `self.On Spawn Limit` true)
                (set `self.Current Enemy` null)
                (break))))
          (if (`self.On Spawn Limit`)
            (`KismetSystemLibrary.Delay` 1.0 :!label _label)
            (`self.Spawn Enemy`)
            (else
              (bind (_randomlocation _returnvalue_6) (`NavigationSystemV1.K2_GetRandomLocationInNavigableRadius` (`self.Teleport Location`) 300.0 null null))
              (if _returnvalue_6
                (bind _returnvalue_7 (`self.K2_TeleportTo` :`self` _current_enemy :`DestLocation` _randomlocation))
                (if _returnvalue_7
                  (`/Game/Blueprints/Enemy/Enemy.Casted Event` _current_enemy)))
              (`KismetSystemLibrary.Delay` 0.2)
              (`self.Spawn Enemy`))))))
    (:`Is Not Valid`
      (goto _label))))

(fn `UserConstructionScript`)